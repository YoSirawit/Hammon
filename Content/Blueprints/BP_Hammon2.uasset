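; BP_Hammon2 is the player actor, with a charge attack, timed parry, HP and checkpoint respawn.
; BP_HammonController events drive charge VFX, cooldown resets and a half-second defense that swaps the sphere material and negates a hit.
; AttackRadius overlaps damage BP_BossCat, and BossMap adds boss health and player HUD widgets.
; Tick advances cooldown timers and, when IsDead is set, respawns it above the last checkpoint.
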(event OnComponentBeginOverlap(AttackRadius)
  (params (OverlappedComponent :type Primitive%20Component%20Object%20Reference) (OtherActor :type Actor%20Object%20Reference) (OtherComp :type Primitive%20Component%20Object%20Reference) (OtherBodyIndex :type Integer) (bFromSweep :type Boolean) (SweepResult :type Hit%20Result%20Structure%20%28by%20ref%29))
  (if (!= OtherActor self)
    (bind _asbp_boss_cat (Utilities|Casting|CastToBP_BossCat OtherActor))
    (Game|Damage|ApplyDamage _asbp_boss_cat (Variables|Default|GetDamage) 0 self)
    (Utilities|FlowControl|Delay 3.0)))

(event Custom|ActivateVFX
  (bind _chargingvfx (Variables|Default|GetChargingVFX))
  ;[0.15 0.15 0.15 0.5] Activate VFX If Charge Complete
  (Utilities|FlowControl|DoOnce false
    (:Completed
      (Components|Activation|Activate (Variables|Default|GetChargeCompleteVFX) true)
      (Development|PrintString "activate VFX" true true "(R=0.070513,G=1.000000,B=0.094693,A=1.000000)")
      (Niagara|ResetSystem _chargingvfx)
      (Components|Activation|Deactivate _chargingvfx))))

(event Custom|DeactivateVFX
  (bind _chargingvfx (Variables|Default|GetChargingVFX))
  ;[0.15 0.15 0.15 0.5] Activate VFX If Charge Complete
  (Components|Activation|Deactivate (Variables|Default|GetChargeCompleteVFX))
  (Utilities|FlowControl|Sequence
    (:then_0
      (Utilities|FlowControl|DoOnce false) ; enters at Reset
    )
    (:then_1
      (Variables|Default|SetATK_CD 0.0))))

(event Custom|ActivateChargingVFX
  (Components|Activation|Activate (Variables|Default|GetChargingVFX) false))

(event Custom|Defense
  (bind _sphere (Variables|Default|GetSphere))
  (Variables|Default|SetDEF_CD 0.0)
  (Variables|Default|SetIsDefending true)
  (Rendering|Material|SetMaterial _sphere 0 "/Game/Characters/Mat_ball_def.Mat_ball_def")
  (Utilities|FlowControl|Delay 0.5)
  (Rendering|Material|SetMaterial _sphere 0 "/Game/Characters/Mat_ball.Mat_ball")
  (Variables|Default|SetIsDefending false))

(event Game|Damage|EventAnyDamage
  (params (Damage :type Float%20%28single-precision%29) (DamageType :type Damage%20Type%20Object%20Reference) (InstigatedBy :type Controller%20Object%20Reference) (DamageCauser :type Actor%20Object%20Reference))
  (if (Variables|Default|GetIsDefending)
    (Variables|Default|SetIsDefending false)
    (Default|CallDefendSuccess)
    (else
      (Variables|Default|SetHP (Math|Float|Clamp(Float) (- (Variables|Default|GetHP) Damage) 0.0 (Variables|Default|GetHP))))))

(event EventBeginPlay
  (bind _returnvalue (Game|GetPlayerController 0))
  ;[0.15 0.15 0.15 0.5] Set Starter Checkpoint
  (Variables|Default|SetLastCheckpoint (Transformation|GetActorTransform))
  ;[0.15 0.15 0.15 0.5] Activate VFX If Charge Complete
  (bind _asbp_hammon_controller (Utilities|Casting|CastToBP_HammonController (Pawn|GetController)))
  (EventDispatchers|BindEventtoChargeMax _asbp_hammon_controller (delegate Custom|ActivateVFX))
  (EventDispatchers|BindEventtoCharging _asbp_hammon_controller (delegate Custom|ActivateChargingVFX))
  (EventDispatchers|BindEventtoAttack _asbp_hammon_controller (delegate Custom|DeactivateVFX))
  (EventDispatchers|BindEventtoDefense _asbp_hammon_controller (delegate Custom|Defense))
  (bind _returnvalue_2 (Game|GetCurrentLevelName true))
  (if (Utilities|Enum|Equal(Enum) _returnvalue_2 "BossMap")
    (bind _returnvalue_3 (UserInterface|CreateWidget "/Game/Characters/BossCat/Behavior/BossHealthBar.BossHealthBar_C" _returnvalue))
    (UserInterface|Viewport|AddtoViewport _returnvalue_3 0)
    (bind _returnvalue_4 (UserInterface|CreateWidget "/Game/Widgets/WBP_PlayerGUI.WBP_PlayerGUI_C" _returnvalue))
    (UserInterface|Viewport|AddtoViewport _returnvalue_4 0)))

(event EventTick
  (params (DeltaSeconds :type Float%20%28single-precision%29))
  (bind _returnvalue (Utilities|Time|GetWorldDeltaSeconds))
  ;[0.15 0.15 0.15 0.5] Set Warp Location & Warp when fall out of map
  (if (not (Variables|Default|GetisDead?))
    _
    (else
      (CallFunction|FellMap)))
  ;[0.15 0.15 0.15 0.5] Track Attack Cooldown
  (Variables|Default|SetATK_CD (+ (Variables|Default|GetATK_CD) _returnvalue))
  (Variables|Default|SetDEF_CD (+ _returnvalue (Variables|Default|GetDEF_CD))))

(fn ConstructionScript)

(fn TakeDamage
  (params (Damage :type Float%20%28double-precision%29))
  (Variables|Default|SetHP (- (Variables|Default|GetHP) Damage)))

(fn NewCheckpoint
  (params (Location :type Transform))
  (Variables|Default|SetLastCheckpoint Location)
  (Development|PrintString "new checkpoint"))

(fn FellMap
  (Transformation|SetActorLocation (+ (.Location (Math|Transform|BreakTransform (Variables|Default|GetLastCheckpoint))) "0.000000,0.000000,1000.000000") false false)
  (Variables|Default|SetisDead? false))