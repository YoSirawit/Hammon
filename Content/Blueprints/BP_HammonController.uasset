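; Player controller for BP_Hammon2 that rolls the pawn's sphere toward the mouse cursor and handles attack, defense and pause input.
; Each tick, a cursor trace drives a planar force that scales with cursor distance, and attack applies the same force at attack acceleration.
; Enhanced Input events fire dispatchers for charge, attack and defense, with delay-based cooldowns and a pausable charging sound.
; Pause opens a widget, switches to UI-only input and pauses the game.
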(event Custom|EnableAttack
  (Variables|Default|SetCanAttack? true))

(event Input|EnhancedActionEvents|EnhancedInputActionIA_Attack
  (params (ActionValue :type Boolean) (ElapsedSeconds :type Float%20%28double-precision%29) (TriggeredSeconds :type Float%20%28double-precision%29) (InputAction :type Input%20Action%20Object%20Reference :default "/Game/Characters/Hammon/IA_Attack.IA_Attack"))
  (:Triggered
    (if (Variables|Default|GetCanAttack?)
      (CallFunction|AddBallForcetoCursor (Variables|Default|GetAttackAcc))
      (Input|SetInputModeGameOnly (Game|GetPlayerController 0) false)
      (Default|CallAttack)
      (Variables|Default|SetCanAttack? false)
      (Utilities|FlowControl|Delay 3.0)
      (Variables|Default|SetCanAttack? true)))
  (:Ongoing
    (if (and (>= ElapsedSeconds 2.0) (Variables|Default|GetCanAttack?))
      (Default|CallChargeMax)
      (Class|AudioComponent|SetPaused (stale _returnvalue) true)
      (else
        (Default|CallCharging)
        (Utilities|FlowControl|Sequence
          (:then_0
            (Utilities|FlowControl|DoOnce false
              (:Completed
                (bind _returnvalue (Audio|SpawnSound2D "/Game/Sound/SFX/Charging_Cue.Charging_Cue" 1.0 1.0 0.0 0))
                (Components|Activation|SetActive _returnvalue true false))))
          (:then_1
            (Class|AudioComponent|SetPaused _returnvalue false))))))
  (:Canceled
    (Default|CallChargeCancled :!label _label)
    (Input|SetInputModeGameOnly (Game|GetPlayerController 0) false)
    (Class|AudioComponent|SetPaused _returnvalue true))
  (:Completed
    (goto _label)))

(event Input|EnhancedActionEvents|EnhancedInputActionIA_Defense
  (params (ActionValue :type Boolean) (ElapsedSeconds :type Float%20%28double-precision%29) (TriggeredSeconds :type Float%20%28double-precision%29) (InputAction :type Input%20Action%20Object%20Reference :default "/Game/Characters/Hammon/IA_Defense.IA_Defense"))
  (:Started
    (if (Variables|Default|GetCanDefense?)
      (Utilities|FlowControl|DoOnce false :!label _label
        (:Completed
          (Default|CallDefense)
          (Input|SetInputModeGameOnly (Game|GetPlayerController 0) false)
          (Variables|Default|SetCanDefense? false)
          (Utilities|FlowControl|Delay 5.0)
          (Variables|Default|SetCanDefense? true)
          (goto _label Reset)))))
  (:Canceled
    (Input|SetInputModeGameOnly (Game|GetPlayerController 0) false :!label _label_2))
  (:Completed
    (goto _label_2)))

(event Input|EnhancedActionEvents|EnhancedInputActionIA_Pause
  (params (ActionValue :type Boolean) (ElapsedSeconds :type Float%20%28double-precision%29) (TriggeredSeconds :type Float%20%28double-precision%29) (InputAction :type Input%20Action%20Object%20Reference :default "/Game/Characters/Hammon/IA_Pause.IA_Pause"))
  (bind _returnvalue (Game|GetPlayerController 0))
  (:Started
    (bind _returnvalue_2 (UserInterface|CreateWidget "/Game/UI/Pause.Pause_C"))
    (UserInterface|Viewport|AddtoViewport _returnvalue_2 0)
    (Variables|/Script/Engine.PlayerController|SetbShowMouseCursor _returnvalue true)
    (Input|SetInputModeUIOnly _returnvalue 0 "DoNotLock" false)
    (Game|SetGamePaused true)))

(event EventBeginPlay
  (bind _returnvalue (PlayerController|LocalPlayerSubsystems|GetEnhancedInputLocalPlayerSubsystem))
  (Utilities|IsValid _returnvalue
    (:Is%20Valid
      (Input|AddMappingContext _returnvalue "/Game/Characters/Hammon/IMP_Hammon.IMP_Hammon" 0 "(bIgnoreAllPressedKeysUntilRelease=True,bForceImmediately=False,bNotifyUserSettings=False)")
      (bind _asbp_hammon_2 (Utilities|Casting|CastToBP_Hammon2 (Game|Player|GetPlayerPawn 0)))
      (Input|SetInputModeGameOnly (Game|GetPlayerController 0) false)
      (Variables|Default|SetbShowMouseCursor true))))

(event EventTick
  (params (DeltaSeconds :type Float%20%28single-precision%29))
  ;[0.15 0.15 0.15 0.5] Move where cursor is at
  (CallFunction|AddBallForcetoCursor (Variables|Default|GetMaxMoveSpeed)))

(fn ConstructionScript)

(fn GetLocationUnderCursor
  (bind _hitresult (Game|Player|GetHitResultUnderCursorbyChannel "TraceTypeQuery1" true))
  (bind (_bblockinghit _binitialoverlap _time _distance _location) (Collision|BreakHitResult _hitresult))
  (return _bblockinghit _location))

(fn Get2DLocation
  (params (Location :type Vector))
  (bind (_x _y) (Math|Vector|BreakVector Location))
  (return (Math|Vector|MakeVector _x _y 0.0)))

(fn AddBallForcetoCursor
  (params (Speed :type Float%20%28double-precision%29))
  (bind (_hit _location) (CallFunction|GetLocationUnderCursor))
  (bind _returnvalue (Game|Player|GetPlayerPawn 0))
  (bind _returnvalue_2 (Transformation|GetActorLocation _returnvalue))
  (bind _returnvalue_3 (- _returnvalue_2 _location))
  (bind (_x _y) (Math|Vector|BreakVector _returnvalue_3))
  (if _hit
    (bind _asbp_hammon_2 (Utilities|Casting|CastToBP_Hammon2 _returnvalue))
    (Physics|AddForce (Variables|/Game/Blueprints/BP_Hammon2.BP_Hammon2_C|GetSphere _asbp_hammon_2) (* (Math|Vector|MakeVector _x _y 0.0) (* Speed -1.0)) "None" false)))