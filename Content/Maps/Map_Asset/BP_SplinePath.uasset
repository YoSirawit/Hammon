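; BP_SplinePath is a map actor that lays a path mesh along an editable spline.
; The construction script destroys existing spline mesh components, then adds one per segment between consecutive SplinePath points.
; Each segment uses the Path mesh on the X forward axis, with query and physics collision, bent to the points' local positions and tangents.
; The event graph has no gameplay logic.
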(event EventBeginPlay)

(event Collision|EventActorBeginOverlap
  (params (OtherActor :type Actor%20Object%20Reference)))

(event EventTick
  (params (DeltaSeconds :type Float%20%28single-precision%29)))

(fn ConstructionScript
  (bind _splinepath (Variables|Default|GetSplinePath))
  (for _array_element (Actor|GetComponentsByClass "/Script/Engine.SplineMeshComponent")
    (Components|DestroyComponent _array_element))
  (for _index (range 0 (- (Spline|GetNumberOfSplinePoints _splinepath) 2))
    (bind _returnvalue (AddComponent|AddSplineMeshComponent false))
    (Collision|SetCollisionEnabled _returnvalue "QueryAndPhysics")
    (SplineMesh|SetForwardAxis _returnvalue "X" true)
    (Components|StaticMesh|SetStaticMesh _returnvalue "/Game/Maps/_GENERATED/iyara/path.path")
    (SplineMesh|SetStartandEnd _returnvalue (Spline|GetLocationatSplinePoint _splinepath _index "Local") (* (Spline|GetTangentatSplinePoint _splinepath _index "Local") 1.0) (Spline|GetLocationatSplinePoint _splinepath (+ _index 1) "Local") (* (Spline|GetTangentatSplinePoint _splinepath (+ _index 1) "Local") 1.0) true :!class /Script/Engine.SplineMeshComponent)))