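; BP_slapWood is a map prop whose Slap component endlessly swings back and forth in pitch.
; On BeginPlay it caches the component's relative rotation and waits a random few seconds, so instances start out of sync.
; A timeline lerps pitch from zero to the cached pitch plus 90 degrees, preserving yaw.
; The Finished event toggles IsReverse to alternate forward and reverse playback with a pause between swings.
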(event EventBeginPlay
  ;[0.15 0.15 0.15 0.5] Cellect Mesh Rotator
  (Variables|Default|SetMeshRotation (Variables|/Script/Engine.SceneComponent|GetRelativeRotation (Variables|Default|Getslap)))
  (Utilities|FlowControl|Delay (Math|Random|RandomFloatinRange 0.0 3.0))
  ;[0.15 0.15 0.15 0.5] Looping SLAP Animation
  (bind _alpha (Timeline|TL_slapRotate PlayFromStart)
    (:Update
      (Transformation|SetRelativeRotation (Variables|Default|Getslap) (Math|Rotator|MakeRotator 0.0 (Math|Float|Lerp 0.0 (+ (.Pitch (Math|Rotator|BreakRotator (Variables|Default|GetMeshRotation))) 9e+01) _alpha) (.Yaw (Math|Rotator|BreakRotator (Variables|Default|GetMeshRotation)))) false false))
    (:Finished
      (if (Variables|Default|GetisReverse)
        (Utilities|FlowControl|Delay 2.0)
        (Variables|Default|SetisReverse false)
        (Timeline|TL_slapRotate PlayFromStart)
        (else
          (Variables|Default|SetisReverse true)
          (Utilities|FlowControl|Delay 1.0)
          (Timeline|TL_slapRotate Reverse))))))

(event Collision|EventActorBeginOverlap
  (params (OtherActor :type Actor%20Object%20Reference)))

(fn ConstructionScript)