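; Boss cat character with health UI, health-based phases up to a rage mode with shorter cooldowns, and a ragdoll death that opens the end cutscene.
; Damage updates the phase and mirrors it to the AI blackboard.
; CallAttack plays montages by AttackType and starts the cooldown, with separate events for projectiles, fanned claw zones and lasers.
; Tick updates UI and cooldown, and interpolates twin eye beams toward the player, sphere-tracing for damage.
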(event Custom|CallAttack
  ;[0.15 0.15 0.15 0.5] Call Attack
  (switch int (Variables|Default|GetAttackType)
    (:1
      (switch int (Math|Random|RandomIntegerinRange 0 3)
        (:0
          (Animation|Montage|PlayMontage (Variables|Default|GetSkeletalMesh self) "/Game/Characters/BossCat/Animation/BossCat_Smash_Montage.BossCat_Smash_Montage" 2.0
            (:then
              (Variables|Default|SetIsOnCooldown true))))
        (:1
          (Animation|Montage|PlayMontage (Variables|Default|GetSkeletalMesh self) "/Game/Characters/BossCat/Animation/SmashRightLeft.SmashRightLeft" 2.0
            (:then
              (Variables|Default|SetIsOnCooldown true))))
        (:2
          (Animation|Montage|PlayMontage (Variables|Default|GetSkeletalMesh self) "/Game/Characters/BossCat/Animation/SmashFakeLeft.SmashFakeLeft" 2.0
            (:then
              (Variables|Default|SetIsOnCooldown true))))
        (:3
          (Animation|Montage|PlayMontage (Variables|Default|GetSkeletalMesh self) "/Game/Characters/BossCat/Animation/SmashFakeRight.SmashFakeRight" 2.0
            (:then
              (Variables|Default|SetIsOnCooldown true))))))
    (:2
      (Development|PrintString "Fire Projectile")
      (Animation|Montage|PlayMontage (Variables|Default|GetSkeletalMesh self) "/Game/Characters/BossCat/Animation/Projectile.Projectile" 2.0
        (:then
          (Variables|Default|SetIsOnCooldown true))))
    (:3
      (Development|PrintString "Launch Claw")
      (Animation|Montage|PlayMontage (Variables|Default|GetSkeletalMesh self) "/Game/Characters/BossCat/Animation/BossCat_Slash.BossCat_Slash" 1.5
        (:then
          (Variables|Default|SetIsOnCooldown true))))
    (:4
      (Development|PrintString "Laser Eye")
      (Animation|Montage|PlayMontage (Variables|Default|GetSkeletalMesh self) "/Game/Characters/BossCat/Animation/BossCat_Laser.BossCat_Laser" 1.2
        (:then
          (Variables|Default|SetIsOnCooldown true)))))
  (Variables|Default|SetCurrentCooldown (* (Variables|Default|GetCooldownMultiply) (Variables|Default|GetBaseCooldown))))

(event Custom|UpdatePhase
  (bind _maxhealth (Variables|Default|GetMaxHealth))
  (bind _currenthealth (Variables|Default|GetCurrentHealth))
  (bind _returnvalue (/ _currenthealth _maxhealth))
  (bind _returnvalue_2 (* _returnvalue 1e+02))
  ;[0.15 0.15 0.15 0.5] Set Phase
  (if (<= _returnvalue_2 3e+01)
    (Variables|Default|SetCurrentPhase 4)
    (Variables|Default|SetCooldownMultiply 0.7)
    (Development|PrintString "Enter Rage Mode !!!")
    (bind _asbp_ai_boss_cat (Utilities|Casting|CastToBP_AI_BossCat (Pawn|GetController)))
    (Class|BlackboardComponent|SetValueasInt (AI|GetBlackboard _asbp_ai_boss_cat) (Utilities|Name|MakeLiteralName "CurrentPhase") 4)
    (elif (<= _returnvalue_2 5e+01)
      (Variables|Default|SetCurrentPhase 3)
      (Variables|Default|SetCooldownMultiply 1.0)
      (Development|PrintString "Enter Phase 3")
      (bind _asbp_ai_boss_cat_2 (Utilities|Casting|CastToBP_AI_BossCat (Pawn|GetController)))
      (Class|BlackboardComponent|SetValueasInt (AI|GetBlackboard _asbp_ai_boss_cat_2) (Utilities|Name|MakeLiteralName "CurrentPhase") 3)
      (elif (<= _returnvalue_2 7e+01)
        (Variables|Default|SetCurrentPhase 2)
        (Variables|Default|SetCooldownMultiply 1.0)
        (Development|PrintString "Enter Phase 2")
        (bind _asbp_ai_boss_cat_3 (Utilities|Casting|CastToBP_AI_BossCat (Pawn|GetController)))
        (Class|BlackboardComponent|SetValueasInt (AI|GetBlackboard _asbp_ai_boss_cat_3) (Utilities|Name|MakeLiteralName "CurrentPhase") 2)
        (elif (> _returnvalue_2 7e+01)
          (Variables|Default|SetCurrentPhase 1)
          (Variables|Default|SetCooldownMultiply 1.0)
          (Development|PrintString "Enter Phase 1")
          (bind _asbp_ai_boss_cat_4 (Utilities|Casting|CastToBP_AI_BossCat (Pawn|GetController)))
          (Class|BlackboardComponent|SetValueasInt (AI|GetBlackboard _asbp_ai_boss_cat_4) (Utilities|Name|MakeLiteralName "CurrentPhase") 1))))))

(event Custom|Die
  ;[0.15 0.15 0.15 0.5] Ragdoll Death
  (bind _asbp_ai_boss_cat (Utilities|Casting|CastToBP_AI_BossCat (Pawn|GetController)))
  (AI|Navigation|StopMovement _asbp_ai_boss_cat)
  (Pawn|Components|CharacterMovement|DisableMovement (Variables|Character|GetCharacterMovement))
  (Components|Animation|SetAnimationMode (Variables|Default|GetSkeletalMesh) "AnimationSingleNode" true)
  (Collision|SetCollisionEnabled (Variables|Collision|GetCapsuleComponent) "NoCollision")
  (Collision|SetCollisionProfileName (Variables|Default|GetSkeletalMesh) "Ragdoll" true :!class /Script/Engine.PrimitiveComponent)
  (Physics|SetSimulatePhysics (Variables|Character|GetMesh) true)
  (Class|PrimitiveComponent|WakeAllRigidBodies (Variables|Character|GetMesh))
  (Physics|AddImpulse (Variables|Character|GetMesh) "0.000000,0.000000,20000.000000" "None" true)
  (Utilities|FlowControl|Delay 3.0)
  (Game|OpenLevel(byName) "EndGameCutsceneMap"))

(event Custom|FireProjectile
  ;[0.15 0.15 0.15 0.5] Fire Projectile
  (Variables|Default|SetHamLocation (Transformation|GetActorLocation (Game|Player|GetPlayerPawn 0)))
  (Variables|Default|SetProjectileSpawn (Transformation|GetSocketLocation (Variables|Default|GetSkeletalMesh) "tete"))
  (bind _output_get (Variables|Default|SetDirectionToHam (Math|Vector|Normalize (- (Variables|Default|GetHamLocation) (Variables|Default|GetProjectileSpawn)))))
  (Game|SpawnActorfromClass "/Game/Characters/BossCat/CatBall.CatBall_C" (Math|Transform|MakeTransform (+ (Variables|Default|GetProjectileSpawn) (Math|Vector|MakeVector 0.0 0.0 2e+01)) (Math|Rotator|MakeRotfromX _output_get)) "Undefined" "MultiplyWithRoot" self self))

(event Custom|DoLaser
  ;[0.15 0.15 0.15 0.5] Start Laser
  (Variables|Default|SetIsFiringLaser true)
  (Variables|Default|SetHamPawn (Game|Player|GetPlayerPawn 0))
  (Utilities|FlowControl|Sequence
    (:then_0
      (bind _returnvalue (Niagara|SpawnSystemAttached "/Game/Characters/BossCat/Animation/BossLaser.BossLaser" (Variables|Default|GetSkeletalMesh) "None" "0, 0, 0" "0, 0, 0" "KeepRelativeOffset" false))
      (Utilities|IsValid _returnvalue
        (:Is%20Valid
          (Variables|Default|SetLaserBeam_L _returnvalue)
          (Variables|Default|SetLaserTimer 0.0)
          (bind _returnvalue_2 (Audio|SpawnSound2D "/Game/Sound/SFX/laser.laser" 1.0 1.0 0.0 0))
          (Variables|Default|SetLaserSound _returnvalue_2))))
    (:then_1
      (bind _returnvalue_3 (Niagara|SpawnSystemAttached "/Game/Characters/BossCat/Animation/BossLaser.BossLaser" (Variables|Default|GetSkeletalMesh) "None" "0, 0, 0" "0, 0, 0" "KeepRelativeOffset" false))
      (Utilities|IsValid _returnvalue_3
        (:Is%20Valid
          (Variables|Default|SetLaserBeam_R _returnvalue_3))))))

(event Custom|DoSlash
  ;[0.15 0.15 0.15 0.5] ClawSlash
  (for _index (range 0 16)
    (if (== (Math|Integer|%(Integer) _index 2) 0)
      (bind _returnvalue (Game|SpawnActorfromClass "/Game/Characters/BossCat/ClawZone.ClawZone_C" (Math|Transform|MakeTransform (- (+ (Transformation|GetActorLocation) (* (Math|Vector|RotateVectorAroundAxis (Transformation|GetActorForwardVector) (- (* (Math|Conversions|ToFloat(Integer) _index) (/ (Variables|Default|GetAngle) (Variables|Default|GetDivideAngle))) 45.0) (Math|Vector|MakeVector 0.0 0.0 1.0)) 2.2e+03)) "0.000000,0.000000,437.000000") (Math|Rotator|MakeRotfromX (Math|Vector|RotateVectorAroundAxis (Transformation|GetActorForwardVector) (- (* (Math|Conversions|ToFloat(Integer) _index) (/ (Variables|Default|GetAngle) (Variables|Default|GetDivideAngle))) 45.0) (Math|Vector|MakeVector 0.0 0.0 1.0))) "50.000000,2.000000,1.000000") "Undefined" "MultiplyWithRoot" self 0))
      (Actor|SetLifeSpan _returnvalue 1.5))))

(event Custom|DontLaser
  ;[0.15 0.15 0.15 0.5] Stop Laser
  (Audio|Components|Audio|Stop (Variables|Default|GetLaserSound))
  (Variables|Default|SetIsFiringLaser false)
  (Variables|Default|SetLaserTimer 0.0)
  (Utilities|IsValid (Variables|Default|GetLaserBeam_L)
    (:Is%20Valid
      (Components|DestroyComponent (Variables|Default|GetLaserBeam_L))
      (Components|DestroyComponent (Variables|Default|GetLaserBeam_R)))))

(event Game|Damage|EventAnyDamage
  (params (Damage :type Float%20%28single-precision%29) (DamageType :type Damage%20Type%20Object%20Reference) (InstigatedBy :type Controller%20Object%20Reference) (DamageCauser :type Actor%20Object%20Reference))
  ;[0.15 0.15 0.15 0.5] Update Phase
  (Variables|Default|SetCurrentHealth (Math|Float|Clamp(Float) (- (Variables|Default|GetCurrentHealth) Damage) 0.0 (Variables|Default|GetMaxHealth)))
  (if (<= (Variables|Default|GetCurrentHealth) 0.0)
    (CallFunction|Die)
    (else
      (Development|PrintString (Utilities|String|ToString(Float) (Variables|Default|GetCurrentHealth)))
      (CallFunction|UpdatePhase))))

(event Collision|EventActorBeginOverlap
  (params (OtherActor :type Actor%20Object%20Reference)))

(event EventTick
  (params (DeltaSeconds :type Float%20%28single-precision%29))
  (bind _laserbeam_l (Variables|Default|GetLaserBeam_L))
  (bind _laserbeam_r (Variables|Default|GetLaserBeam_R))
  (bind _health_ui (Variables|Default|GetHealth%20UI))
  ;[0.15 0.15 0.15 0.5] HealthBarUI
  (Utilities|FlowControl|Sequence
    (:then_0
      (Progress|SetPercent (Variables|/Game/Characters/BossCat/Behavior/BossHealthBar.BossHealthBar_C|GetHealthBar _health_ui) (/ (Variables|Default|GetCurrentHealth) 1e+02))
      (if (Variables|Default|GetIsOnCooldown)
        (bind _output_get (Variables|Default|SetCurrentCooldown (- (Variables|Default|GetCurrentCooldown) (Utilities|Time|GetWorldDeltaSeconds))))
        (Rendering|Components|TextRender|SetText (Variables|/Game/Characters/BossCat/Behavior/BossHealthBar.BossHealthBar_C|GetCD_Count _health_ui) (Utilities|Text|ToText(Float) _output_get "HalfToEven"))
        (if (<= (Variables|Default|GetCurrentCooldown) 0.0)
          (Variables|Default|SetIsOnCooldown false))))
    (:then_1
      ;[0.15 0.15 0.15 0.5] Laser Finding
      (if (Variables|Default|GetIsFiringLaser)
        (Variables|Default|SetLaserTimer (+ (Utilities|Time|GetWorldDeltaSeconds) (Variables|Default|GetLaserTimer)))
        (if (>= (Variables|Default|GetLaserTimer) (Variables|Default|GetLaserDuration))
          (CallFunction|DontLaser)
          (else
            (bind _output_get_2 (Variables|Default|SetLaserEnd (Transformation|GetActorLocation (Variables|Default|GetHamPawn))))
            (Variables|Default|SetCurrentLaserEnd (Math|Interpolation|VInterpTo (Variables|Default|GetCurrentLaserEnd) _output_get_2 (Utilities|Time|GetWorldDeltaSeconds) (Variables|Default|GetLaserSpeed)))
            (Utilities|IsValid (Variables|Default|GetLaserBeam_L)
              (:Is%20Valid
                (Niagara|SetNiagaraVariable(Vector3) _laserbeam_l "BeamStart" (Transformation|GetSocketLocation (Variables|Default|GetSkeletalMesh) "eye_L"))
                (Niagara|SetNiagaraVariable(Vector3) _laserbeam_l "BeamEnd" (Variables|Default|GetCurrentLaserEnd))
                (Niagara|SetNiagaraVariable(Vector3) _laserbeam_r "BeamStart" (Transformation|GetSocketLocation (Variables|Default|GetSkeletalMesh) "eye_R"))
                (Niagara|SetNiagaraVariable(Vector3) _laserbeam_r "BeamEnd" (Variables|Default|GetCurrentLaserEnd))
                (bind (_outhit _returnvalue) (Collision|SphereTraceByChannel (Transformation|GetSocketLocation (Variables|Character|GetMesh) "eye_L") (Variables|Default|GetCurrentLaserEnd) 5e+01 "TraceTypeQuery3" false 0 "None"))
                (if _returnvalue
                  (bind _asbp_hammon_2 (Utilities|Casting|CastToBP_Hammon2 (.HitActor (Collision|BreakHitResult _outhit))))
                  (Game|Damage|ApplyDamage _asbp_hammon_2 (* (Utilities|Time|GetWorldDeltaSeconds) 2e+01) 0 0))))))))))

(event EventBeginPlay
  ;[0.15 0.15 0.15 0.5] HealthBarUI
  (bind _returnvalue (UserInterface|CreateWidget "/Game/Characters/BossCat/Behavior/BossHealthBar.BossHealthBar_C" (Game|GetPlayerController 0)))
  (UserInterface|Viewport|AddtoViewport _returnvalue 0)
  (Variables|Default|SetHealth%20UI _returnvalue)
  (Variables|Default|SetCurrentHealth (Variables|Default|GetMaxHealth))
  (Variables|Default|SetCurrentPhase 1)
  (Variables|Default|SetCooldownMultiply 1.0)
  (bind _asbp_ai_boss_cat (Utilities|Casting|CastToBP_AI_BossCat (Pawn|GetController)))
  (Class|BlackboardComponent|SetValueasInt (AI|GetBlackboard _asbp_ai_boss_cat) (Utilities|Name|MakeLiteralName "CurrentPhase") 1))

(fn ConstructionScript)